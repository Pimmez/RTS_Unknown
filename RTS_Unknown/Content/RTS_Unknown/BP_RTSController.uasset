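; Player controller for a multiplayer RTS, handling selection, unit orders, resources, the main UI and team start spawning.
; Left click selects own-team buildings and drives HUD selection; right click sends HUD-selected units to move or work resource nodes.
; Orders and unit production pass through server events, with production deducting unit cost before queueing at the building.
; On authority, player setup spawns the team's center building and starting units.
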(event Custom|ServerPassThrough:UnitMoveCommand
  (params (Unit :type Actor%20Object%20Reference) (Location :type Vector))
  ;[0.3296 1 0.9834] RightClick Server Pass Through Functions
  (Class|ISelection|UnitMoveCommand(Message) Unit Location))

(event Custom|ServerAddUnitToQueue
  (params (Building :type BP%20Parent%20Building%20Class%20Object%20Reference) (Unit :type BP%20Parent%20Unit%20Class%20Reference))
  ;[1 1 1] Produce units
  (Utilities|DeductUnitResourceCost Unit
    (:NotEnoughResources
      (CallFunction|ClientShow:NotEnoughResources))
    (:DeductedResources
      (Default|AddUnittoQueue Building Unit))))

(event Custom|ServerPassThrough:SetIsWorking
  (params (Unit :type Actor%20Object%20Reference) (ResourceNode :type Actor%20Object%20Reference))
  ;[0.3296 1 0.9834] RightClick Server Pass Through Functions
  (Class|IResources|SetIsWorking(Message) Unit ResourceNode))

(event Custom|ServerPassThrough:SetNotWorking
  (params (Unit :type Actor%20Object%20Reference))
  ;[0.3296 1 0.9834] RightClick Server Pass Through Functions
  (Class|IResources|SetNotWorking(Message) Unit))

(event Custom|ClientShow:NotEnoughResources
  (Default|NotEnoughResourcesMessage (Variables|Default|GetMainUI_Widget)))

(event EventTick
  (params (DeltaSeconds :type Float%20%28single-precision%29))
  ;[1 1 1] EVENT TICK + LeftMouseClick
  (if (Variables|Default|GetisLeftMousePressed?)
    (Class|ISelection|SelectionHeld(Message) (HUD|GetHUD))))

(event EventBeginPlay
  ;[1 1 1] Begin Play
  (if (Pawn|IsLocalPlayerController)
    (Utilities|FlowControl|Sequence
      (:then_0
        (Utilities|SetupGameModeandMouse))
      (:then_1
        (Utilities|CreateMainUIWidget)))))

(event EventAddUnittoSelectedUnitArea
  (params (SelectedUnitWidget :type User%20Widget%20Object%20Reference))
  ;[1 1 1] Add unit to selection area
  (Class|HorizontalBox|AddChildtoHorizontalBox (Variables|/Game/RTS_Unknown/Widgets/WBP_MainUI.WBP_MainUI_C|GetUnitBox (Variables|Default|GetMainUI_Widget)) SelectedUnitWidget))

(event EventProduceUnit
  (params (Building :type BP%20Parent%20Building%20Class%20Object%20Reference) (Unit :type BP%20Parent%20Unit%20Class%20Reference))
  ;[1 1 1] Produce units
  (CallFunction|ServerAddUnittoQueue Building Unit))

(event EventIncrementResourceAmount
  (params (Amount :type Integer))
  ;[1 1 1] Increment Resource amount
  (Variables|Default|SetResourceAmount (+ Amount (Variables|Default|GetResourceAmount))))

(event EventClearSelectedBuilding
  ;[1 1 1] Clear Selected Building
  (Utilities|IsValid (Variables|Default|GetSelectedBuilding)
    (:Is%20Valid
      (Class|ISelection|DeselectThis(Message) (Variables|Default|GetSelectedBuilding))
      (Variables|Default|SetSelectedBuilding 0))))

(event EventSetupPlayerStart
  (params (PlayerStartCamp :type BP%20Player%20Start%20Camp%20Object%20Reference) (TeamNumber :type Integer) (TeamColor :type Linear%20Color%20Structure))
  ;[1 1 1] Setup player start
  (Networking|SwitchHasAuthority
    (:Authority
      (Variables|Default|SetTeam%20Number TeamNumber)
      (Variables|Default|SetTeam%20Color TeamColor)
      (Utilities|InitializePlayerSpawn PlayerStartCamp))))

(event Input|MouseEvents|LeftMouseButton
  (params (Key :type Key%20Structure :default "None"))
  (bind _returnvalue (HUD|GetHUD))
  ;[1 1 1] EVENT TICK + LeftMouseClick
  (:Pressed
    (Variables|Default|SetisLeftMousePressed? true)
    (Utilities|HandleBuildingClick)
    (Class|ISelection|SelectionPressed(Message) _returnvalue))
  (:Released
    (Variables|Default|SetisLeftMousePressed? false)
    (Class|ISelection|SelectionReleased(Message) _returnvalue)))

(event Input|MouseEvents|RightMouseButton
  (params (Key :type Key%20Structure :default "None"))
  (bind (_location _hitactor) (Utilities|RightClickHitResultUnderCursor))
  ;[1 1 1] RightMouseButton
  (:Pressed
    (if (== (Utilities|GetClass _hitactor) "/Game/RTS_Unknown/Resources/BP_ResourceNode.BP_ResourceNode_C")
      (Utilities|HandleRightClickResourceNode _hitactor)
      (else
        (Utilities|HandleRightClicktoMoveUnits _location)))))

(fn ConstructionScript)

(fn Moveto
  (params (Location :type Vector))
  (AI|Navigation|SimpleMovetoLocation self Location)
  (Niagara|SpawnSystematLocation (Variables|Input|GetFXCursor) Location))

(fn Follow
  (params (Location :type Vector))
  (bind _returnvalue (Pawn|GetControlledPawn))
  (Pawn|Input|AddMovementInput _returnvalue (Math|Vector|GetUnitDirection(Vector) (Transformation|GetActorLocation _returnvalue) Location) 1.0 false))

(fn GetLocationUnderCursor
  (bind _hitresult (Game|Player|GetHitResultUnderCursorbyChannel "TraceTypeQuery1" true))
  (bind (_bblockinghit _binitialoverlap _time _distance _location) (Collision|BreakHitResult _hitresult))
  (return _bblockinghit _location))

(fn GetLocationUnderFinger
  (bind _hitresult (Class|PlayerController|GetHitResultUnderFingerbyChannel "Touch1" "TraceTypeQuery1" false))
  (bind (_bblockinghit _binitialoverlap _time _distance _location) (Collision|BreakHitResult _hitresult))
  (return _bblockinghit _location))

(fn GetResourceAmount
  (return (Variables|Default|GetResourceAmount)))

(fn GetTeam
  (return 0))

(fn GrabSelectedUnits
  (return 0))

(fn IsonMyTeam?
  (params (TeamNumber :type Integer))
  (return (== TeamNumber (Variables|Default|GetTeam%20Number))))