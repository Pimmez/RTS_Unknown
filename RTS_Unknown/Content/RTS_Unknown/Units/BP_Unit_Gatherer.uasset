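; RTS gatherer unit that shuttles between a resource node and a same-team drop-off building to earn resources for its player.
; SetIsWorking stores the node and searches team buildings for the nearest drop-off.
; Collect runs a timer before sending the unit to drop off, and DropOff credits the team's controller and sends it back.
; Multicast events sync particles, audio and the nose material showing cargo, while Tick spins the team-colored Spinner.
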(event Custom|ResourceCollector
  ;[1 1 1] Collect Resource
  ;;[1 1 1] Collect resource overtime
  (Utilities|Time|ClearandInvalidateTimerbyHandle (Variables|Default|GetResourceCollectTimer))
  (Variables|Default|SetHasResource? true)
  ;;[1 1 1] Move to dropoff
  (CallFunction|UnitMoveCommand (Transformation|GetActorLocation (Variables|Default|GetDropOffBuilding)))
  ;;[1 1 1] Multicast done collecting sound and effects
  (CallFunction|MulticastDoneCollecting))

(event Custom|MulticastStartCollecting
  ;[1 1 1] Collect Resource
  ;;[1 1 1] Multicast start collecting sound and effects
  (Components|Activation|SetActive (Variables|Default|GetParticleSystem) true false)
  (Audio|Components|Audio|Play (Variables|Default|GetAudio) 0.0))

(event Custom|MulticastDoneCollecting
  ;[1 1 1] Collect Resource
  ;;[1 1 1] Multicast done collecting sound and effects
  (Components|Activation|SetActive (Variables|Default|GetParticleSystem) false false)
  (Audio|Components|Audio|Stop (Variables|Default|GetAudio))
  (Rendering|Material|SetMaterial (Variables|Default|GetNose) 0 "/Game/StarterContent/Materials/M_Metal_Gold.M_Metal_Gold"))

(event Custom|MulticastResourceDroppedOff
  ;[1 1 1] Dropoff Resource
  ;;[1 1 1] Multicast Resources dropped off
  (Rendering|Material|SetMaterial (Variables|Default|GetNose) 0 "/Game/StarterContent/Materials/M_Basic_Wall.M_Basic_Wall"))

(event Custom|MulticastNotWorking
  ;[1 1 1] Set Gatherer on not working
  ;;[1 1 1] Multicast not working sound and effects
  (Components|Activation|SetActive (Variables|Default|GetParticleSystem) false false)
  (Audio|Components|Audio|Stop (Variables|Default|GetAudio)))

(event EventTick
  (params (DeltaSeconds :type Float%20%28single-precision%29))
  ;[1 1 1] Event Tick
  (Transformation|AddRelativeRotation (Variables|Default|GetSpinner) (Math|Rotator|MakeRotator 0.0 0.0 (* DeltaSeconds 2.5e+02)) false false))

(event EventSetIsWorking
  (params (ResourceNode :type Actor%20Object%20Reference))
  ;[1 1 1] Set Gatherer is working
  (Variables|Default|SetisWorking? true)
  (Variables|Default|SetResourceNode ResourceNode)
  ;;[1 1 1] Find nearest dropoff point
  (bind _outactors (Actor|GetAllActorsOfClass "/Game/RTS_Unknown/Buildings/BP_ParentBuildingClass.BP_ParentBuildingClass_C"))
  (for _array_element _outactors
    (bind _teamnumber (Default|GetTeam _array_element))
    (if (== _teamnumber (Variables|Default|GetTeamNumber))
      (if (< (Transformation|GetDistanceTo _array_element self) (Variables|Default|GetClosestDropOffBuildingDistance))
        (Variables|Default|SetDropOffBuilding _array_element)
        (Variables|Default|SetClosestDropOffBuildingDistance (Transformation|GetDistanceTo _array_element self)))))
  ;;[1 1 1] Move to next target
  (if (Variables|Default|GetHasResource?)
    (CallFunction|UnitMoveCommand (Transformation|GetActorLocation (Variables|Default|GetDropOffBuilding)))
    (else
      (CallFunction|UnitMoveCommand (Transformation|GetActorLocation (Variables|Default|GetResourceNode))))))

(event EventSetNotWorking
  ;[1 1 1] Set Gatherer on not working
  (Variables|Default|SetisWorking? false)
  (Utilities|Time|ClearandInvalidateTimerbyHandle (Variables|Default|GetResourceCollectTimer))
  ;;[1 1 1] Multicast not working sound and effects
  (CallFunction|MulticastNotWorking))

(event EventCollect
  ;[1 1 1] Collect Resource
  (if (Variables|Default|GetisWorking?)
    ;;[1 1 1] Already has resource, head to dropoff
    (if (Variables|Default|GetHasResource?)
      (CallFunction|UnitMoveCommand (Transformation|GetActorLocation (Variables|Default|GetDropOffBuilding)))
      (else
        ;;[1 1 1] Check if collection already has started
        (if (not (Utilities|Time|IsValidTimerHandle (Variables|Default|GetResourceCollectTimer)))
          ;;[1 1 1] Stop movement
          (CallFunction|UnitMoveCommand (Transformation|GetActorLocation))
          ;;[1 1 1] Multicast start collecting sound and effects
          (CallFunction|MulticastStartCollecting)
          ;;[1 1 1] Collect resource overtime
          (bind _returnvalue (Utilities|Time|SetTimerbyEvent (delegate Custom|ResourceCollector) 4.0))
          (Variables|Default|SetResourceCollectTimer _returnvalue))))))

(event EventDropOff
  ;[1 1 1] Dropoff Resource
  (if (Variables|Default|GetisWorking?)
    ;;[1 1 1] No resources, go back to resourcenode
    (if (Variables|Default|GetHasResource?)
      ;;[1 1 1] Increment resource amount
      (Class|IResources|IncrementResourceAmount(Message) (Game|GetPlayerController (Variables|Default|GetTeamNumber)) 10)
      (Variables|Default|SetHasResource? false)
      ;;[1 1 1] Multicast Resources dropped off
      (CallFunction|MulticastResourceDroppedOff)
      ;;[1 1 1] Move to resource node
      (CallFunction|UnitMoveCommand (Transformation|GetActorLocation (Variables|Default|GetResourceNode)))
      (else
        (CallFunction|UnitMoveCommand (Transformation|GetActorLocation (Variables|Default|GetResourceNode)))))))

(fn ConstructionScript
  (bind _meshesforteamcoloring (Variables|Default|GetMeshesForTeamColoring))
  (|CallParentFunction)
  (Utilities|Array|Add _meshesforteamcoloring (Variables|Default|GetBody))
  (Utilities|Array|Add _meshesforteamcoloring (Variables|Default|GetSpinner)))

(fn GetResourceAmount
  (return 0))