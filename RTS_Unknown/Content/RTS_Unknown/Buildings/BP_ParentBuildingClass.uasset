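; Base RTS building actor that handles selection, team coloring and server-side unit production.
; BeginPlay creates the selection widget with action buttons, shown alongside a decal on select, and tints mesh and minimap dynamic materials by team.
; A looping authority timer pulls queued unit classes, accumulates their default production time, then spawns them with the team's number and color.
; Server overlaps send DropOffMessage to the other actor; IsOnMyTeam is a stub returning false.
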(event Custom|AddUnitToQueue
  (params (Unit :type BP%20Parent%20Unit%20Class%20Reference))
  (Utilities|Array|Add (Variables|Default|GetUnitProductionQueue) Unit))

(event Custom|ProcessProductionQueue
  ;[1 1 1] Unit Porduction
  (if (Variables|Default|GetisProducingUnits?)
    (bind _output_get (Variables|Default|SetProductionTimeSpend (+ (Variables|Default|GetProductionTimeSpend) (Variables|Default|GetProductionTimer))))
    (bind _output_get_2 (Variables|Default|SetProductionProgress (/ _output_get (Variables|Default|GetProductionTimeNeeded))))
    (if (>= _output_get_2 1.0)
      (Game|SpawnActorfromClass (Variables|Default|GetUnitBeingProduced) (Math|Transform|MakeTransform (Transformation|GetWorldLocation (Variables|Default|GetUnit%20Spawn%20Point)) "0, 0, 0" "1.000000,1.000000,1.000000") "AdjustIfPossibleButAlwaysSpawn" 0 (Variables|Default|GetTeamNumber) (Variables|Default|GetTeamColor) 0)
      (Variables|Default|SetProductionProgress 0.0)
      (Variables|Default|SetProductionTimeSpend 0.0)
      (Variables|Default|SetUnitBeingProduced 0)
      (Variables|Default|SetisProducingUnits? false))
    (elif (> (Utilities|Array|Length (Variables|Default|GetUnitProductionQueue)) 0)
      (bind _output_get_3 (Variables|Default|SetUnitBeingProduced (Utilities|Array|Get(acopy) (Variables|Default|GetUnitProductionQueue))))
      (Variables|Default|SetProductionTimeNeeded (.ProductionTime (Utilities|GetClassDefaults _output_get_3)))
      (Utilities|Array|RemoveIndex (Variables|Default|GetUnitProductionQueue))
      (Variables|Default|SetisProducingUnits? true))))

(event Collision|EventActorBeginOverlap
  (params (OtherActor :type Actor%20Object%20Reference))
  (Networking|SwitchHasAuthority
    (:Authority
      (Class|IResources|DropOff(Message) OtherActor))))

(event EventSetToolTip
  (params (ToolTipWidget :type User%20Widget%20Object%20Reference))
  (bind _buildingselected_widget (Variables|Default|GetBuildingSelected_Widget))
  (bind _tooltipbox (Variables|/Game/RTS_Unknown/Widgets/WBP_SelectedBuilding.WBP_SelectedBuilding_C|GetTooltipBox _buildingselected_widget))
  ;[1 1 1] Set Tooltip
  (Widget|Panel|ClearChildren _tooltipbox)
  (Utilities|IsValid ToolTipWidget
    (:Is%20Valid
      (Class|HorizontalBox|AddChildtoHorizontalBox _tooltipbox ToolTipWidget))))

(event EventDeselectThis
  (Rendering|SetVisibility (Variables|Default|GetSelectiveDecal) false false)
  (Widget|RemovefromParent (Variables|Default|GetBuildingSelected_Widget)))

(event EventSelectThis
  (Rendering|SetVisibility (Variables|Default|GetSelectiveDecal) true false)
  (UserInterface|Viewport|AddtoViewport (Variables|Default|GetBuildingSelected_Widget) 0))

(event EventBeginPlay
  (Utilities|FlowControl|Sequence
    (:then_0
      ;[1 1 1] Create building selected widget
      (bind _returnvalue (UserInterface|CreateWidget "/Game/RTS_Unknown/Widgets/WBP_SelectedBuilding.WBP_SelectedBuilding_C"))
      (Variables|Default|SetBuildingSelected_Widget _returnvalue)
      (Variables|/Game/RTS_Unknown/Widgets/WBP_SelectedBuilding.WBP_SelectedBuilding_C|SetBuildingReference _returnvalue self)
      (for _array_element (Variables|Default|GetActionBoxButtons)
        (Class|WrapBox|AddChildtoWrapBox (Variables|/Game/RTS_Unknown/Widgets/WBP_SelectedBuilding.WBP_SelectedBuilding_C|GetAction_Wrapbox (Variables|Default|GetBuildingSelected_Widget)) _array_element)))
    (:then_1
      ;[1 1 1] Setup Teamcolor
      (bind _returnvalue_2 (Rendering|Material|CreateDynamicMaterialInstance (Rendering|Material|GetMaterial (Variables|Default|GetBuildingMesh) 0) "None" "None" :!class /Script/Engine.KismetMaterialLibrary))
      (Rendering|Material|SetVectorParameterValue _returnvalue_2 "TeamColor" (Variables|Default|GetTeamColor) :!class /Script/Engine.MaterialInstanceDynamic)
      (Rendering|Material|SetMaterial (Variables|Default|GetBuildingMesh) 0 _returnvalue_2)
      (bind _returnvalue_3 (Rendering|Material|CreateDynamicMaterialInstance "/Game/RTS_Unknown/Materials/M_Minimap.M_Minimap" "None" "None" :!class /Script/Engine.KismetMaterialLibrary))
      (Rendering|Material|SetVectorParameterValue _returnvalue_3 "TeamColor" (Variables|Default|GetTeamColor) :!class /Script/Engine.MaterialInstanceDynamic)
      (Rendering|Material|SetMaterial (Variables|Default|GetBP_MinimapComponent) 0 _returnvalue_3))
    (:then_2
      ;[1 1 1] Unit Porduction
      (Networking|SwitchHasAuthority
        (:Authority
          (Utilities|Time|SetTimerbyEvent (delegate Custom|ProcessProductionQueue) (Variables|Default|GetProductionTimer) true))))))

(fn ConstructionScript)

(fn GetTeam
  (return (Variables|Default|GetTeamNumber)))

(fn GrabSelectedUnits
  (return 0))

(fn IsonMyTeam?
  (params (TeamNumber :type Integer))
  (return false))